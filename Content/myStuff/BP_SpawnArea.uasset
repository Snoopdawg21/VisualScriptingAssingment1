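; BP_SpawnArea is a spawn zone actor that relocates among level actors tagged "SpawnLocation".
; On BeginPlay it caches those tagged actors in an array, in the order the query returns them.
; Each MoveSpawnZone call, not triggered within this Blueprint, teleports it to the current entry and advances the index.
; The index wraps on a hardcoded twelve-location limit instead of the array's length.
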(event `self.ReceiveBeginPlay`
  (bind _outactors (`GameplayStatics.GetAllActorsWithTag` "SpawnLocation"))
  (bind _output_get (set `self.spawnLocations` _outactors)))

(fn `MoveSpawnZone`
  (`self.K2_SetActorLocation` (`self.K2_GetActorLocation` (`|GetArrayItem` (`self.spawnLocations`) (`self.locationNum`))) false true)
  (if (>= (`self.locationNum`) 11)
    (set `self.locationNum` 0)
    (else
      (`/Engine/EditorBlueprintResources/StandardMacros.IncrementInt` (`self.locationNum`)))))

(fn `UserConstructionScript`)