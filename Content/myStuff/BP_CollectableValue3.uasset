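; BP_CollectableValue3 is a pickup worth three points that the player collects by walking into it.
; On BeginPlay it caches the third-person game mode and player character and sets its value.
; When the player overlaps its Box, it reports the value to the game mode, asks it to spawn a collectable passing itself, then destroys itself.
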(event `self.ReceiveBeginPlay`
  (bind _asbp_third_person_game_mode (cast `/Game/ThirdPerson/Blueprints/BP_ThirdPersonGameMode` (`GameplayStatics.GetGameMode`)))
  (set `self.GameMode` _asbp_third_person_game_mode)
  (bind _asbp_third_person_character (cast `/Game/ThirdPerson/Blueprints/BP_ThirdPersonCharacter` (`GameplayStatics.GetPlayerPawn` 0)))
  (set `self.Player` _asbp_third_person_character)
  (set `self.Value` 3))

(event `self.Box.OnComponentBeginOverlap`
  (params (OverlappedComponent :type "PrimitiveComponent Object Reference") (OtherActor :type "Actor Object Reference") (OtherComp :type "PrimitiveComponent Object Reference") (OtherBodyIndex :type Integer) (bFromSweep :type Boolean) (SweepResult :type "HitResult Structure (by ref)"))
  (if (== OtherActor (`self.Player`))
    (`/Game/ThirdPerson/Blueprints/BP_ThirdPersonGameMode.Collect` (`self.GameMode`) (`self.Value`))
    (`/Game/ThirdPerson/Blueprints/BP_ThirdPersonGameMode.SpawnCollectable` (`self.GameMode`) self)
    (`self.K2_DestroyActor`)))

(fn `UserConstructionScript`)